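; Enemy character Blueprint that patrols back and forth between two points supplied through the Setdestination event.
; A FlipFlop alternates the AI MoveTo target, and each successful arrival triggers a timeline-driven 180-degree yaw turn from the current rotation before the next move starts.
; The construction script snaps the Rifle to the mesh's Weapon socket.
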(event Custom|Set%20destination
  (params (Dest1 :type Vector) (Dest2 :type Vector))
  (Variables|Default|SetDest1 Dest1)
  (Variables|Default|SetDest2 Dest2)
  (CallFunction|Move))

(event Custom|Move
  (Utilities|FlowControl|FlipFlop
    (:A
      (Variables|Default|SetDestination (Variables|Default|GetDest1)))
    (:B
      (Variables|Default|SetDestination (Variables|Default|GetDest2))))
  (AI|AIMoveTo self (Variables|Default|GetDestination) 0 3.0 false
    (:OnSuccess
      (CallFunction|Turn))))

(event Custom|Turn
  (Variables|Default|SetstartRotation (Transformation|GetActorRotation))
  (bind _angle (Timeline|Angle PlayFromStart)
    (:Update
      (Transformation|SetActorRotation (Math|Rotator|MakeRotator 0.0 0.0 (+ (Math|Float|Lerp 0.0 1.8e+02 _angle) (.yaw (Variables|Default|GetstartRotation))))))
    (:Finished
      (CallFunction|Move))))

(event EventBeginPlay)

(fn ConstructionScript
  (Transformation|AttachComponentToComponent (Variables|Default|GetRifle) (Variables|Character|GetMesh) "Weapon" "SnapToTarget" "SnapToTarget" "SnapToTarget" true))