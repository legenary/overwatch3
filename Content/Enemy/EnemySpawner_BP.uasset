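; Enemy respawn manager that replaces dead enemies with the same class at the transform their death dispatcher reports, after a short delay.
; On BeginPlay it binds death dispatchers on every placed Enemy_Parent_BP, with roaming enemies also reporting two destinations into shared variables.
; Respawned roaming enemies receive those stored destinations.
; Respawned roaming and standing enemies rebind their death dispatcher to continue the cycle, but not the roaming destination dispatcher.
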(event Custom|Call%20Respawn
  (params (Class :type Enemy%20Parent%20BP%20Class%20Reference) (Transform :type Transform))
  (CallFunction|Respawn Class Transform))

(event Custom|Respawn
  (params (Class :type Enemy%20Parent%20BP%20Class%20Reference) (Transform :type Transform))
  (bind (_location _rotation) (Math|Transform|BreakTransform Transform))
  (Utilities|FlowControl|Delay 2.0)
  (bind _returnvalue (AI|SpawnAIFromClass Class 0 _location _rotation false 0))
  (Utilities|FlowControl|Sequence
    (:then_0
      (bind _asenemy_roaming_bp (Utilities|Casting|CastToEnemy_Roaming_BP _returnvalue))
      (Default|SetDestination _asenemy_roaming_bp (Variables|Default|GetDest1) (Variables|Default|GetDest2))
      (EventDispatchers|BindEventtoEnemyDeathDispatcher _asenemy_roaming_bp (delegate Custom|EnemyDeathDispatcher_Event_0)))
    (:then_1
      (bind _asenemy_standing_bp (Utilities|Casting|CastToEnemy_Standing_BP _returnvalue))
      (EventDispatchers|BindEventtoEnemyDeathDispatcher _asenemy_standing_bp (delegate Custom|EnemyDeathDispatcher_Event_0)))))

(event Custom|Assign%20Dest
  (params (Dest1 :type Vector) (Dest2 :type Vector))
  (Variables|Default|SetDest1 Dest1)
  (Variables|Default|SetDest2 Dest2))

(event Custom|EnemyDeathDispatcher_Event_0
  (params (Class :type Enemy%20Parent%20BP%20Class%20Reference) (Transform :type Transform))
  (CallFunction|Respawn Class Transform))

(event EventBeginPlay
  (bind _outactors (Actor|GetAllActorsOfClass "/Game/Enemy/Enemy_Parent_BP.Enemy_Parent_BP_C"))
  (for _array_element _outactors
    (EventDispatchers|AssignEnemyDeathDispatcher _array_element (delegate Custom|Call%20Respawn))
    (bind _asenemy_roaming_bp (Utilities|Casting|CastToEnemy_Roaming_BP _array_element))
    (EventDispatchers|AssignRoamingEnemyDeathDispatcher _asenemy_roaming_bp (delegate Custom|Assign%20Dest))))

(event Collision|EventActorBeginOverlap
  (params (OtherActor :type Actor%20Object%20Reference)))

(event EventTick
  (params (DeltaSeconds :type Float%20%28single-precision%29)))

(fn ConstructionScript)