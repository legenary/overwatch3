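; Enemy actor that fires three-shot bursts at intervals while it has the player in sight.
; PawnSensing sets the sight flag and stores the seen character, and a retriggerable delay clears both shortly after sightings stop.
; Tick accumulates time to pace bursts, each a delayed loop calling Fire on the Weapon_BP child actor with a destructable projectile.
; The construction script snaps that rifle to the mesh's Weapon socket.
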(event OnSeePawn(PawnSensing)
  (params (Pawn :type Pawn%20Object%20Reference))
  (Utilities|FlowControl|Sequence
    (:then_0
      (bind _asfirst_person_character (Utilities|Casting|CastToFirstPersonCharacter Pawn))
      (Variables|Default|SetplayerInSight true)
      (Variables|Default|SetSeen%20Player _asfirst_person_character))
    (:then_1
      (Utilities|FlowControl|RetriggerableDelay 1.1)
      (Variables|Default|SetplayerInSight false)
      (Variables|Default|SetSeen%20Player 0))))

(event Custom|Three%20fires
  (Utilities|ForLoopwithDelay 1 3 0.5
    (:Loop%20body
      (CallFunction|FireWeapon "/Game/FirstPersonBP/Blueprints/FirstPersonProjectile_Destructable.FirstPersonProjectile_Destructable_C"))))

(event EventBeginPlay)

(event Collision|EventActorBeginOverlap
  (params (OtherActor :type Actor%20Object%20Reference)))

(event EventTick
  (params (DeltaSeconds :type Float%20%28single-precision%29))
  (if (Variables|Default|GetplayerInSight)
    (if (== (Variables|Default|GettimeFromLastFire) 0.0)
      (CallFunction|ThreeFires))
    (bind _output_get (Variables|Default|SettimeFromLastFire (+ DeltaSeconds (Variables|Default|GettimeFromLastFire))))
    (if (>= _output_get (Variables|Default|GettimeBetweenFire))
      (Variables|Default|SettimeFromLastFire 0.0))))

(fn ConstructionScript
  (Transformation|AttachComponentToComponent (Variables|Default|GetRifle) (Variables|Character|GetMesh) "Weapon" "SnapToTarget" "SnapToTarget" "SnapToTarget" true))

(fn FireWeapon
  (params (ProjectileClass :type First%20Person%20Projectile%20Class%20Reference))
  (bind _asweapon_bp (Utilities|Casting|CastToWeapon_BP (Variables|/Script/Engine.ChildActorComponent|GetChildActor (Variables|Default|GetRifle))))
  (Default|Fire _asweapon_bp ProjectileClass))