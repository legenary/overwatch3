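; Parent enemy Blueprint with a health bar widget and a child-actor rifle snapped to the mesh's Weapon socket during construction.
; BeginPlay caches the widget, and UpdateHealth sets its bar from HP over MaxHP, running only at startup within this file.
; A radius component shows the bar while a FirstPersonCharacter overlaps it and hides it on exit.
; FireWeapon forwards its parameter to the rifle's Weapon_BP Fire function.
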(event OnComponentBeginOverlap(HealthBarRadius)
  (params (OverlappedComponent :type Primitive%20Component%20Object%20Reference) (OtherActor :type Actor%20Object%20Reference) (OtherComp :type Primitive%20Component%20Object%20Reference) (OtherBodyIndex :type Integer) (bFromSweep :type Boolean) (SweepResult :type Hit%20Result%20Structure%20%28by%20ref%29))
  (Utilities|Casting|CastToFirstPersonCharacter OtherActor)
  (Rendering|SetVisibility (Variables|Default|GetHealthBar) true false))

(event OnComponentEndOverlap(HealthBarRadius)
  (params (OverlappedComponent :type Primitive%20Component%20Object%20Reference) (OtherActor :type Actor%20Object%20Reference) (OtherComp :type Primitive%20Component%20Object%20Reference) (OtherBodyIndex :type Integer))
  (Utilities|Casting|CastToFirstPersonCharacter OtherActor)
  (Rendering|SetVisibility (Variables|Default|GetHealthBar) false false))

(event EventBeginPlay
  (bind _asenemy_health_bar_ui (Utilities|Casting|CastToEnemy_HealthBar_UI (UserInterface|GetUserWidgetObject (Variables|Default|GetHealthBar))))
  (Variables|Default|SetHealthBarRef _asenemy_health_bar_ui)
  (CallFunction|UpdateHealth))

(event EventTick
  (params (DeltaSeconds :type Float%20%28single-precision%29)))

(fn ConstructionScript
  (Transformation|AttachComponentToComponent (Variables|Default|GetRifle) (Variables|Character|GetMesh) "Weapon" "SnapToTarget" "SnapToTarget" "SnapToTarget" true))

(fn FireWeapon
  (params (NewParam :type First%20Person%20Projectile%20Class%20Reference))
  (bind _asweapon_bp (Utilities|Casting|CastToWeapon_BP (Variables|/Script/Engine.ChildActorComponent|GetChildActor (Variables|Default|GetRifle))))
  (Default|Fire _asweapon_bp NewParam))

(fn UpdateHealth
  (Progress|SetPercent (Variables|/Game/Enemy/Enemy_HealthBar_UI.Enemy_HealthBar_UI_C|GetHPbar (Variables|Default|GetHealthBarRef)) (/ (Variables|Default|GetHP) (Variables|Default|GetmaxHP))))