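; Standing enemy Blueprint that fires destructible projectiles while it has the player in sight.
; PawnSensing flags a seen FirstPersonCharacter as the target, and a retriggerable delay clears it shortly after sightings stop.
; While the player is in sight, Tick runs a timer that calls ThreeFires once per fire interval.
; Despite its name, ThreeFires currently fires one shot, as its delayed loop has a single iteration.
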(event OnSeePawn(PawnSensing)
  (params (Pawn :type Pawn%20Object%20Reference))
  (Utilities|FlowControl|Sequence
    (:then_0
      (bind _asfirst_person_character (Utilities|Casting|CastToFirstPersonCharacter Pawn))
      (Variables|Default|SetplayerInSight true)
      (Variables|Default|SetseenPlayer _asfirst_person_character))
    (:then_1
      (Utilities|FlowControl|RetriggerableDelay 1.1)
      (Variables|Default|SetplayerInSight false)
      (Variables|Default|SetseenPlayer 0))))

(event Custom|Three%20fires
  (Utilities|ForLoopwithDelay 1 1 0.8
    (:Loop%20body
      (CallFunction|FireWeapon "/Game/FirstPersonBP/Blueprints/FirstPersonProjectile_Destructable.FirstPersonProjectile_Destructable_C"))))

(event EventBeginPlay
  (|CallParentFunction) ; This node is disabled and will not be called.\nDrag off pins to build functionality.
)

(event Collision|EventActorBeginOverlap
  (params (OtherActor :type Actor%20Object%20Reference))
  (|CallParentFunction OtherActor) ; This node is disabled and will not be called.\nDrag off pins to build functionality.
)

(event EventTick
  (params (DeltaSeconds :type Float%20%28single-precision%29))
  (|CallParentFunction DeltaSeconds)
  (if (Variables|Default|GetplayerInSight)
    (if (== (Variables|Default|GettimeFromLastFire) 0.0)
      (CallFunction|ThreeFires))
    (bind _output_get (Variables|Default|SettimeFromLastFire (+ DeltaSeconds (Variables|Default|GettimeFromLastFire))))
    (if (>= _output_get (Variables|Default|GettimeBetweenFire))
      (Variables|Default|SettimeFromLastFire 0.0))))

(fn ConstructionScript
  (|CallParentFunction))