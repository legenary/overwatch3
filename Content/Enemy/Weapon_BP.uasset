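; Enemy rifle actor that fires a projectile of the class passed to its Fire event and plays a gunshot sound.
; The projectile spawns at the Muzzle socket, aimed along the right vector of the component its child actor component is attached to.
; A debug-drawn line trace also runs from the muzzle along the weapon's own right vector, but its hit result does not affect the shot.
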(event Custom|Fire
  (params (ProjectileClass :type First%20Person%20Projectile%20Class%20Reference))
  (bind _rifle (Variables|Default|GetRifle))
  (bind _rifle_2 (Variables|Default|GetRifle))
  (bind _returnvalue (Transformation|GetSocketLocation _rifle "Muzzle"))
  (bind _returnvalue_2 (Transformation|GetSocketLocation _rifle_2 "Muzzle"))
  (bind (_outhit _returnvalue_3) (Collision|LineTraceByChannel _returnvalue (+ (* (Transformation|GetActorRightVector) 4e+03) _returnvalue) "TraceTypeQuery1" false 0 "ForDuration"))
  (Game|SpawnActorfromClass ProjectileClass (Math|Transform|MakeTransform _returnvalue_2 (Math|Rotator|FindLookatRotation _returnvalue_2 (+ (Math|Vector|GetRightVector (Transformation|GetAttachParent (Class|Actor|GetParentComponent))) _returnvalue_2))) "AdjustIfPossibleButDontSpawnIfColliding" self 0) ; Spawn projectile
  (Audio|PlaySoundatLocation "/Game/FirstPerson/Audio/FirstPersonTemplateWeaponFire02.FirstPersonTemplateWeaponFire02" "0, 0, 0" "0, 0, 0" 1.0 1.0 0.0 0 0 0))

(fn ConstructionScript)