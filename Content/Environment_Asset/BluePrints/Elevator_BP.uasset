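; Elevator Blueprint that moves its base mesh vertically when something overlaps its trigger box.
; Construction script stores the mesh's relative Z as the start height and its negation as the end height.
; After a short delay, overlap plays a timeline whose Rise track lerps between these heights at a fixed Y offset.
; Leaving the trigger reverses the timeline after a longer delay, with no filtering on the overlapping actor.
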(event OnComponentBeginOverlap(TriggerBox)
  (params (OverlappedComponent :type Primitive%20Component%20Object%20Reference) (OtherActor :type Actor%20Object%20Reference) (OtherComp :type Primitive%20Component%20Object%20Reference) (OtherBodyIndex :type Integer) (bFromSweep :type Boolean) (SweepResult :type Hit%20Result%20Structure%20%28by%20ref%29))
  (Utilities|FlowControl|Delay 0.3)
  (bind _rise (Timeline|Timeline_0 Play)
    (:Update
      (Transformation|SetRelativeLocation (Variables|Default|GetElevatorBase_SM) (Math|Vector|MakeVector 0.0 2e+02 (Math|Float|Lerp (Variables|Default|GetBegin) (Variables|Default|GetEnd) _rise)) false false))))

(event OnComponentEndOverlap(TriggerBox)
  (params (OverlappedComponent :type Primitive%20Component%20Object%20Reference) (OtherActor :type Actor%20Object%20Reference) (OtherComp :type Primitive%20Component%20Object%20Reference) (OtherBodyIndex :type Integer))
  (Utilities|FlowControl|Delay 1.0)
  (bind _rise (Timeline|Timeline_0 Reverse)
    (:Update
      (Transformation|SetRelativeLocation (Variables|Default|GetElevatorBase_SM) (Math|Vector|MakeVector 0.0 2e+02 (Math|Float|Lerp (Variables|Default|GetBegin) (Variables|Default|GetEnd) _rise)) false false))))

(fn ConstructionScript
  (bind _elevatorbase_sm (Variables|Default|GetElevatorBase_SM))
  (bind _relativelocation (Variables|/Script/Engine.SceneComponent|GetRelativeLocation _elevatorbase_sm))
  (Variables|Default|SetBegin (.z _relativelocation))
  (Variables|Default|SetEnd (* -1 (.z _relativelocation))))