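; Health pack pickup that bobs and spins, healing a FirstPersonCharacter that walks into its sphere.
; Tick drives a timeline that offsets the mesh from its construction-time height and adds yaw.
; A successful AddHealthBy hides and deactivates the pack for a short delay, while failure prints "Health Full".
; On respawn it re-enters the pickup logic through a custom event if the character still overlaps.
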(event OnComponentBeginOverlap(Sphere)
  (params (OverlappedComponent :type Primitive%20Component%20Object%20Reference) (OtherActor :type Actor%20Object%20Reference) (OtherComp :type Primitive%20Component%20Object%20Reference) (OtherBodyIndex :type Integer) (bFromSweep :type Boolean) (SweepResult :type Hit%20Result%20Structure%20%28by%20ref%29))
  ;[1 1 1] Character walk on health pack
  (if (Variables|Default|GetActive?)
    (bind _asfirst_person_character (Utilities|Casting|CastToFirstPersonCharacter OtherActor))
    (bind _return (Default|AddHealthby _asfirst_person_character (Variables|Default|GetHealthValue)))
    (if _return
      (Rendering|SetVisibility (Variables|Default|GetHealthPack_SM) false false)
      (Variables|Default|SetActive? false)
      (Utilities|FlowControl|Delay 2.0)
      (Rendering|SetVisibility (Variables|Default|GetHealthPack_SM) true false)
      (Variables|Default|SetActive? true)
      ;[1 1 1] If character still on health pack
      (bind _returnvalue (Actor|GetActorOfClass "/Game/FirstPersonBP/Blueprints/FirstPersonCharacter.FirstPersonCharacter_C"))
      (if (Collision|IsOverlappingActor (Variables|Default|GetSphere) _returnvalue :!class /Script/Engine.PrimitiveComponent)
        (CallFunction|CharacterOverlapping))
      (else
        (Development|PrintString "Health Full")))))

(event Custom|CharacterOverlapping
  ;[1 1 1] Character walk on health pack
  (if (Variables|Default|GetActive?)
    (bind _asfirst_person_character (Utilities|Casting|CastToFirstPersonCharacter (stale OnComponentBeginOverlap(Sphere) OtherActor)))
    (bind _return (Default|AddHealthby _asfirst_person_character (Variables|Default|GetHealthValue)))
    (if _return
      (Rendering|SetVisibility (Variables|Default|GetHealthPack_SM) false false)
      (Variables|Default|SetActive? false)
      (Utilities|FlowControl|Delay 2.0)
      (Rendering|SetVisibility (Variables|Default|GetHealthPack_SM) true false)
      (Variables|Default|SetActive? true)
      ;[1 1 1] If character still on health pack
      (bind _returnvalue (Actor|GetActorOfClass "/Game/FirstPersonBP/Blueprints/FirstPersonCharacter.FirstPersonCharacter_C"))
      (if (Collision|IsOverlappingActor (Variables|Default|GetSphere) _returnvalue :!class /Script/Engine.PrimitiveComponent)
        (CallFunction|CharacterOverlapping))
      (else
        (Development|PrintString "Health Full")))))

(event EventTick
  (params (DeltaSeconds :type Float%20%28single-precision%29))
  ;[1 1 1] Self motion
  (bind _healthpackheightoffset (Timeline|Timeline_0 Play)
    (:Update
      (Components|Timeline|SetPlayRate (Variables|Default|GetTimeline_0) 0.6)
      (Transformation|SetRelativeTransform (Variables|Default|GetHealthPack_SM) (Math|Transform|MakeTransform (Math|Vector|MakeVector 0.0 0.0 (+ (* _healthpackheightoffset 7.0) (Variables|Default|GetHealthPackHeight))) (Math|Rotator|MakeRotator 0.0 0.0 (+ 0.6 (.yaw (Variables|/Script/Engine.SceneComponent|GetRelativeRotation (Variables|Default|GetHealthPack_SM))))) "1,1,1") false false))))

(fn ConstructionScript
  (Variables|Default|SetHealthPackHeight (.z (Variables|/Script/Engine.SceneComponent|GetRelativeLocation (Variables|Default|GetHealthPack_SM)))))