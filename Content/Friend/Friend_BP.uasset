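; Friendly AI companion that shoots enemies it sees and runs back to the player when it strays too far.
; Tick sets a Panicking flag when the player is beyond a set distance and, while set, issues AI move-to requests toward the player, clearing it on arrival.
; When not panicking, PawnSensing sightings of Enemy_BP turn the actor to face the target and fire the socket-attached child-actor rifle.
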(event OnSeePawn(PawnSensing)
  (params (Pawn :type Pawn%20Object%20Reference))
  (if (not (Variables|Default|Getpanicking))
    (bind _asenemy_bp (Utilities|Casting|CastToEnemy_BP Pawn))
    (CallFunction|FireWeaponat _asenemy_bp)
    (Development|PrintString "Fire")))

(event EventBeginPlay)

(event Collision|EventActorBeginOverlap
  (params (OtherActor :type Actor%20Object%20Reference)))

(event EventTick
  (params (DeltaSeconds :type Float%20%28single-precision%29))
  (Utilities|FlowControl|Sequence
    (:then_0
      (if (Variables|Default|Getpanicking)
        (bind _returnvalue (Actor|GetActorOfClass "/Game/FirstPersonBP/Blueprints/FirstPersonCharacter.FirstPersonCharacter_C"))
        (AI|AIMoveTo self "0, 0, 0" _returnvalue 1.5e+02 false
          (:OnSuccess
            (Variables|Default|Setpanicking false)))))
    (:then_1
      (bind _res (CallFunction|IsinPanicRange))
      (if _res
        (Variables|Default|Setpanicking true)))))

(fn ConstructionScript
  (Transformation|AttachComponentToComponent (Variables|Default|GetRifle) (Variables|Character|GetMesh) "Weapon" "SnapToTarget" "SnapToTarget" "SnapToTarget" true)
  (bind _res (CallFunction|IsinPanicRange))
  (Variables|Default|Setpanicking _res))

(fn FireWeaponat
  (params (FireTarget :type Enemy%20BP%20Object%20Reference))
  (CallFunction|Faceat FireTarget)
  (bind _asweapon_bp (Utilities|Casting|CastToWeapon_BP (Variables|/Script/Engine.ChildActorComponent|GetChildActor (Variables|Default|GetRifle))))
  (Default|Fire _asweapon_bp))

(fn IsinPanicRange
  (bind _returnvalue (Actor|GetActorOfClass "/Game/FirstPersonBP/Blueprints/FirstPersonCharacter.FirstPersonCharacter_C"))
  (return (> (Math|Vector|VectorLength (- (Transformation|GetActorLocation _returnvalue) (Transformation|GetActorLocation self))) 4e+02)))

(fn Faceat
  (params (FaceAtTarget :type Character%20Object%20Reference))
  (Transformation|SetActorRotation (Math|Rotator|FindLookatRotation (Transformation|GetActorLocation self) (Transformation|GetActorLocation FaceAtTarget))))